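; HotelRoomState tracks the grid position of a pod in the Burlington Hotel age and handles requests to move it.
; A move to new coordinates, accepted only while the pod is idle, fakes travel with a sound and a 30-second delay, then dings and updates the stored position.
; On arrival it checks whether the pod rests over the linking book's coordinates, currently only logging the result.
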(event `self.ReceiveBeginPlay`)

(event `self.ReceiveTick`
  (params (DeltaSeconds :type "Float (single-precision)")))

(event `PodMoveRequested`
  (params (DestinationX :type Integer) (DestinationY :type Integer))
  ;[1 1 1] give the illusion of a moving pod with sound, then change the position
  (bind _matched (`self.CoordinatesMatch` DestinationX DestinationY (`self.PodPositionX`) (`self.PodPositionY`)))
  (if _matched
    _
    (elif (not (`self.PodIsMoving`))
      (set `self.PodIsMoving` true)
      (`GameplayStatics.PlaySound2D` "/Game/Content/Shared/Sound/Effects/PodMove.PodMove" 1.5)
      (`KismetSystemLibrary.Delay` 30.0)
      (`GameplayStatics.PlaySound2D` "/Game/Content/Shared/Sound/Effects/ding.ding")
      (`self.SetPodPosition` DestinationX DestinationY)
      (set `self.PodIsMoving` false)
      (bind _overlinkingbook (`self.IsStoppedOverLinkingBook`))
      (if _overlinkingbook
        (`KismetSystemLibrary.PrintString` "POD IS OVER LINKINGBOOK" false)
        (else
          (`KismetSystemLibrary.PrintString` "POD IS NOWHERE INTERESTING" false))))))

(fn `CoordinatesMatch`
  (params (X :type Integer) (Y :type Integer) (A :type Integer) (B :type Integer))
  (returns (Matched :type Boolean))
  (return (and (== X A) (== Y B))))

(fn `IsStoppedOverLinkingBook`
  (returns (OverLinkingBook :type Boolean))
  (bind _matched (`self.CoordinatesMatch` (`self.PodPositionX`) (`self.PodPositionY`) (`self.LinkingBookPositionX`) (`self.LinkingBookPositionY`)))
  (return (and _matched (not (`self.PodIsMoving`)))))

(fn `SetPodPosition`
  (params (CoordinateX :type Integer) (CoordinateY :type Integer))
  (set `self.PodPositionX` CoordinateX)
  (set `self.PodPositionY` CoordinateY)
  (`KismetSystemLibrary.PrintString` (`KismetStringLibrary.Concat_StrStr` "POD ARRIVED AT " (`KismetStringLibrary.Conv_IntToString` CoordinateX) ", " (`KismetStringLibrary.Conv_IntToString` CoordinateY)) false true (struct :`R` 0.240349 :`G` 0.79 :`A` 1.0)))

(fn `UserConstructionScript`)