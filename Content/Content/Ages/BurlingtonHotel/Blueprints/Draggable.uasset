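; Base actor for mouse-draggable props, with a configurable mesh and materials set in the construction script.
; Clicking the mesh starts a hold; past a short time threshold, Tick moves the actor to the cursor trace's XY, keeping its Z.
; Tick polls the left button to fire ManualOnRelease, working around the unreliable OnReleased event.
; Hand cursors reflect hover and grab, while child classes can read QuickClick to distinguish clicks from drags.
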(event `self.ReceiveTick`
  (params (DeltaSeconds :type "Float (single-precision)"))
  (bind _returnvalue (`GameplayStatics.GetPlayerController` 0))
  (bind _returnvalue_2 (`KismetMathLibrary.MakeVector` (.x (`.Location` (`GameplayStatics.BreakHitResult` (`PlayerController.GetHitResultUnderCursorByChannel` _returnvalue "TraceTypeQuery1" false)))) (.y (`.Location` (`GameplayStatics.BreakHitResult` (`PlayerController.GetHitResultUnderCursorByChannel` _returnvalue "TraceTypeQuery1" false)))) (.z (`self.K2_GetActorLocation`))))
  (if (not (`self.disableDrag`))
    ;[1 1 1] Manually perform an OnRelease event (cannot depend on the engine's)
    (bind _mouse_is_held_down (`self.DetermineIfMouseHeldDown`))
    (if _mouse_is_held_down
      (set `self.isHeldThisTick` true)
      (else
        (set `self.isHeldThisTick` false)))
    (if (`self.mouseHeldDownOnDraggableMesh`)
      (if (and (`self.wasHeldLastTick`) (not (`self.isHeldThisTick`)))
        ;;[1 1 1] OnRelease (do this here -- the actual event was not firing properly)
        (`self.ManualOnRelease`) ; kept around so the children inheriting can use it
        (set `self.mouseHeldDownOnDraggableMesh` false)
        (`self.SetCursor` "Default")))
    (set `self.wasHeldLastTick` (`self.isHeldThisTick`))
    ;[1 1 1] Logic for detemining if merely clicking, or dragging
    (if (`self.mouseHeldDownOnDraggableMesh`)
      (bind _isadrag (`self.DetermineIfADrag` 0.5))
      (if _isadrag
        (set `self.quickClick` false)
        ;[1 1 1] move actor according to mouse drag movement
        (set `PlayerController.CurrentMouseCursor` "GrabHandClosed" _returnvalue)
        (if (not (< (`KismetMathLibrary.VSize` (- (`self.previousLocation`) _returnvalue_2)) 0.5))
          (`self.SetLocation` _returnvalue_2)
          (set `self.previousLocation` _returnvalue_2))
        (else
          (set `self.quickClick` true))))))

(event `self.DraggableMesh.OnClicked`
  (params (TouchedComponent :type "PrimitiveComponent Object Reference"))
  ;[1 1 1] toggle dragging mode with a click
  (set `self.mouseHeldDownOnDraggableMesh` true)
  (`self.SetCursor` "GrabHandClosed"))

(event `self.DraggableMesh.OnReleased`
  (params (TouchedComponent :type "PrimitiveComponent Object Reference"))
  ;[1 1 1] make inactive when dragging stops --- utterly useless, doesn't work reliably
  (set `self.mouseHeldDownOnDraggableMesh` false :!label _label)
  (`self.SetCursor` "GrabHand"))

(event `ManualOnRelease`
  ;[1 1 1] make inactive when dragging stops --- utterly useless, doesn't work reliably
  (goto _label))

(event `self.DraggableMesh.OnBeginCursorOver`
  (params (TouchedComponent :type "PrimitiveComponent Object Reference"))
  ;[1 1 1] Handle cursor roll over/off
  (if (not (`self.mouseHeldDownOnDraggableMesh`))
    (`self.SetCursor` "GrabHand")))

(event `self.DraggableMesh.OnEndCursorOver`
  (params (TouchedComponent :type "PrimitiveComponent Object Reference"))
  ;[1 1 1] Handle cursor roll over/off
  (if (not (`self.mouseHeldDownOnDraggableMesh`))
    (`self.SetCursor` "Default")))

(fn `DetermineIfADrag`
  (params (timeBeforeConsideredDrag :type "Float (double-precision)"))
  (returns (IsADrag :type Boolean))
  (return (< timeBeforeConsideredDrag (`PlayerController.GetInputKeyTimeDown` (`GameplayStatics.GetPlayerController` 0) "LeftMouseButton"))))

(fn `DetermineIfMouseHeldDown`
  (returns (`mouse is held down` :type Boolean))
  (return (> (`PlayerController.GetInputKeyTimeDown` (`GameplayStatics.GetPlayerController` 0) "LeftMouseButton") 0.0)))

(fn `GetQuickClick`
  (returns (QuickClick :type Boolean))
  (return (`self.quickClick`)))

(fn `SetCursor`
  (params (Cursor :type "EMouseCursor Enum"))
  (set `PlayerController.CurrentMouseCursor` Cursor (`GameplayStatics.GetPlayerController` 0)))

(fn `SetLocation`
  (params (NewLocation :type "Vector Structure"))
  (`self.K2_SetActorLocation` NewLocation))

(fn `UserConstructionScript`
  (bind _draggablemesh (`self.DraggableMesh`))
  (`StaticMeshComponent.SetStaticMesh` _draggablemesh (`self.CustomMesh`))
  (`PrimitiveComponent.SetMaterial` _draggablemesh 0 (`self.CustomMaterial1`))
  (`PrimitiveComponent.SetMaterial` _draggablemesh 1 (`self.CustomMaterial2`)))