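; SliderKnob is a draggable knob actor for the Burlington Hotel Age, meant to move with its X position locked.
; The construction script caches the actor's starting X as LockedAxisPosition.
; On Tick, after the parent's tick, while MouseHeldDownOnDraggableMesh is true it restores that X, keeping current Y and Z.
; That world position is rotated by the actor's rotation before being applied as the new location.
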(event `self.ReceiveBeginPlay`)

(event `self.ReceiveActorBeginOverlap`
  (params (OtherActor :type "Actor Object Reference")))

(event `self.ReceiveTick`
  (params (DeltaSeconds :type "Float (single-precision)"))
  (bind (_returnvalue_x _returnvalue_y _returnvalue_z) (`KismetMathLibrary.BreakVector` (`self.K2_GetActorLocation`)))
  (`parent.ReceiveTick` 0.0)
  (if (`self.mouseHeldDownOnDraggableMesh`)
    (`self.SetLocation` (`KismetMathLibrary.GreaterGreater_VectorRotator` (`KismetMathLibrary.MakeVector` (`self.lockedAxisPosition`) _returnvalue_y _returnvalue_z) (`self.K2_GetActorRotation`)))))

(fn `UserConstructionScript`
  (bind _returnvalue_x (`KismetMathLibrary.BreakVector` (`self.K2_GetActorLocation`)))
  (`parent.UserConstructionScript`)
  (set `self.lockedAxisPosition` _returnvalue_x))